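; BPC_MasterMonster is a monster character, named as a master class, that moves on request and hurts the player hero on contact.
; The FollowPlayer event feeds a supplied world direction into movement input, leaving the choice of direction to the caller.
; When the HitBox begins overlapping an actor that casts to BPC_Player_Hero, it applies a small fixed amount of damage to that hero.
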(event `Follow Player`
  (params (WorldDirection :type "Vector Structure"))
  (`self.AddMovementInput` WorldDirection))

(event `self.HitBox.OnComponentBeginOverlap`
  (params (OverlappedComponent :type "PrimitiveComponent Object Reference") (OtherActor :type "Actor Object Reference") (OtherComp :type "PrimitiveComponent Object Reference") (OtherBodyIndex :type Integer) (bFromSweep :type Boolean) (SweepResult :type "HitResult Structure (by ref)"))
  (bind _asbpc_player_hero (cast `/Game/Game25D/Blueprint/Characters/Hero/BPC_Player_Hero` OtherActor))
  (`GameplayStatics.ApplyDamage` _asbpc_player_hero 1.0))

(fn `UserConstructionScript`
  (`parent.UserConstructionScript`))