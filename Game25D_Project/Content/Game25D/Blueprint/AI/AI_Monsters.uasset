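; AI controller for monsters in the 25D game that makes them chase the first player's pawn.
; On possess it casts the pawn to BPC_MasterMonster and stores it, and on BeginPlay it caches the player pawn.
; Each Tick it passes the forward vector of the look-at rotation from monster to player into the monster's FollowPlayer, with no pathfinding in this graph.
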(event `self.ReceiveBeginPlay`
  (set `self.Player` (`GameplayStatics.GetPlayerPawn` 0)))

(event `self.ReceiveTick`
  (params (DeltaSeconds :type "Float (single-precision)"))
  (`/Game/Game25D/Blueprint/Characters/BPC_MasterMonster.Follow Player` (stale `self.ReceivePossess` _output_get) (`KismetMathLibrary.GetForwardVector` (`KismetMathLibrary.FindLookAtRotation` (`self.K2_GetActorLocation` (`self.Possesed Pawn`)) (`self.K2_GetActorLocation` (`self.Player`))))))

(event `self.ReceivePossess`
  (params (PossessedPawn :type "Pawn Object Reference"))
  (bind _asbpc_master_monster (cast `/Game/Game25D/Blueprint/Characters/BPC_MasterMonster` PossessedPawn))
  (bind _output_get (set `self.Possesed Pawn` _asbpc_master_monster)))

(fn `UserConstructionScript`)